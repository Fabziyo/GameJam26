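; BP_Geist is a ghost pawn for a triggered apparition, starting hidden with collision disabled.
; SetTriggerOnWorkspace arms it by enabling collision on the capsule and two trigger boxes.
; When a BPI_Player actor enters either box, the mesh appears and AIMoveTo sends it to a hardcoded location.
; On arrival it hides, disables its collision and, after a short delay, calls Toilette on BP_MasterManager.
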(event OnComponentBeginOverlap(Box)
  (params (OverlappedComponent :type Primitive%20Component%20Object%20Reference) (OtherActor :type Actor%20Object%20Reference) (OtherComp :type Primitive%20Component%20Object%20Reference) (OtherBodyIndex :type Integer) (bFromSweep :type Boolean) (SweepResult :type Hit%20Result%20Structure%20%28by%20ref%29))
  (bind _mesh (Variables|Character|GetMesh))
  ;[0.15 0.15 0.15 0.5] Trigger for both Sides
  (if (Utilities|DoesObjectImplementInterface OtherActor "/Game/Blueprints/Interfaces/BPI_Player.BPI_Player_C")
    (Rendering|SetVisibility _mesh true false)
    (Collision|SetCollisionEnabled _mesh "NoCollision")
    (AI|AIMoveTo self "-440.000000,1050.000000,88.000000" 0 5.0 false
      (:OnSuccess
        (Rendering|SetVisibility (Variables|Character|GetMesh) false false)
        (Collision|SetCollisionEnabled (Variables|Collision|GetCapsuleComponent) "NoCollision")
        (Collision|SetCollisionEnabled (Variables|Default|GetBox) "NoCollision")
        (Collision|SetCollisionEnabled (Variables|Default|GetBox1) "NoCollision")
        (Utilities|FlowControl|Delay 0.25)
        (bind _returnvalue (Actor|GetActorOfClass "/Game/Blueprints/BP_MasterManager.BP_MasterManager_C"))
        (Default|Toilette _returnvalue)))))

(event OnComponentBeginOverlap(Box1)
  (params (OverlappedComponent :type Primitive%20Component%20Object%20Reference) (OtherActor :type Actor%20Object%20Reference) (OtherComp :type Primitive%20Component%20Object%20Reference) (OtherBodyIndex :type Integer) (bFromSweep :type Boolean) (SweepResult :type Hit%20Result%20Structure%20%28by%20ref%29))
  (bind _mesh (Variables|Character|GetMesh))
  ;[0.15 0.15 0.15 0.5] Trigger for both Sides
  (if (Utilities|DoesObjectImplementInterface OtherActor "/Game/Blueprints/Interfaces/BPI_Player.BPI_Player_C")
    (Rendering|SetVisibility _mesh true false)
    (Collision|SetCollisionEnabled _mesh "NoCollision")
    (AI|AIMoveTo self "-440.000000,1050.000000,88.000000" 0 5.0 false
      (:OnSuccess
        (Rendering|SetVisibility (Variables|Character|GetMesh) false false)
        (Collision|SetCollisionEnabled (Variables|Collision|GetCapsuleComponent) "NoCollision")
        (Collision|SetCollisionEnabled (Variables|Default|GetBox) "NoCollision")
        (Collision|SetCollisionEnabled (Variables|Default|GetBox1) "NoCollision")
        (Utilities|FlowControl|Delay 0.25)
        (bind _returnvalue (Actor|GetActorOfClass "/Game/Blueprints/BP_MasterManager.BP_MasterManager_C"))
        (Default|Toilette _returnvalue)))))

(event Custom|Set%20Trigger%20On%20Workspace
  ;[0.15 0.15 0.15 0.5] Set Trigger On
  (Collision|SetCollisionEnabled (Variables|Collision|GetCapsuleComponent) "QueryAndPhysics")
  (Collision|SetCollisionEnabled (Variables|Default|GetBox) "QueryAndPhysics")
  (Collision|SetCollisionEnabled (Variables|Default|GetBox1) "QueryAndPhysics")
  (Development|PrintText "Hello"))

(event EventBeginPlay
  ;[0.15 0.15 0.15 0.5] Set Trigger Off and Ghost
  (Variables|Default|SetPlayer%20Ref (Game|GetPlayerCharacter 0))
  (Rendering|SetVisibility (Variables|Character|GetMesh) false false)
  (Collision|SetCollisionEnabled (Variables|Character|GetMesh) "NoCollision")
  (Collision|SetCollisionEnabled (Variables|Collision|GetCapsuleComponent) "NoCollision")
  (Collision|SetCollisionEnabled (Variables|Default|GetBox) "NoCollision")
  (Collision|SetCollisionEnabled (Variables|Default|GetBox1) "NoCollision"))

(event Collision|EventActorBeginOverlap
  (params (OtherActor :type Actor%20Object%20Reference)))

(event EventTick
  (params (DeltaSeconds :type Float%20%28single-precision%29)))

(fn ConstructionScript)