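; Game-end ghost ("Geist") that stays hidden until the player enters its trigger box, then appears with sound.
; BeginPlay hides the mesh and disables its collision, while the capsule keeps query and physics collision.
; A box overlap by any BPI_Player implementer shows the mesh, enables its collision and plays the FMOD audio.
; Nothing re-hides the ghost or latches the trigger, so re-entering calls Play again.
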(event OnComponentBeginOverlap(Box)
  (params (OverlappedComponent :type Primitive%20Component%20Object%20Reference) (OtherActor :type Actor%20Object%20Reference) (OtherComp :type Primitive%20Component%20Object%20Reference) (OtherBodyIndex :type Integer) (bFromSweep :type Boolean) (SweepResult :type Hit%20Result%20Structure%20%28by%20ref%29))
  (bind _mesh (Variables|Character|GetMesh))
  ;[0.15 0.15 0.15 0.5] Trigger for both Sides
  (if (Utilities|DoesObjectImplementInterface OtherActor "/Game/Blueprints/Interfaces/BPI_Player.BPI_Player_C")
    (Rendering|SetVisibility _mesh true false)
    (Collision|SetCollisionEnabled _mesh "QueryAndPhysics")
    (Class|FMODAudioComponent|Play (Variables|Default|GetFMODAudio))))

(event EventBeginPlay
  ;[0.15 0.15 0.15 0.5] Set Trigger Off and Ghost
  (Variables|Default|SetPlayer%20Ref (Game|GetPlayerCharacter 0))
  (Rendering|SetVisibility (Variables|Character|GetMesh) false false)
  (Collision|SetCollisionEnabled (Variables|Character|GetMesh) "NoCollision")
  (Collision|SetCollisionEnabled (Variables|Collision|GetCapsuleComponent) "QueryAndPhysics"))

(event Collision|EventActorBeginOverlap
  (params (OtherActor :type Actor%20Object%20Reference)))

(event EventTick
  (params (DeltaSeconds :type Float%20%28single-precision%29)))

(fn ConstructionScript)