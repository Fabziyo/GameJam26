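; BP_Printer is an interactable printer that starts out malfunctioning, shaking and playing high-pitched FMOD audio from BeginPlay.
; A Wiggle timeline rocks the root's rotation back and forth while the audio plays.
; Interact, gated by a Fixed flag, notifies BP_MasterManager through FixedPrinters, stops both effects and resets rotation.
; Approach and Leave toggle a highlight overlay material, shown only until it is interacted with.
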(event Custom|WiggleHorror
  (bind _fmodaudio (Variables|Default|GetFMODAudio))
  (Variables|Default|SetCanInteract true)
  (Class|FMODAudioComponent|SetPitch _fmodaudio 1.5)
  (Class|FMODAudioComponent|Play _fmodaudio)
  (if (not (Variables|Default|GetInteracted))
    (bind _alpha (Timeline|Wiggle Play)
      (:Update
        (Transformation|SetRelativeRotation (Variables|Default|GetDefaultSceneRoot) (Math|Rotator|Lerp(Rotator) "0.000000,0.000000,2.000000" "0.000000,0.000000,-2.000000" _alpha) false false)))))

(event EventBeginPlay
  (CallFunction|WiggleHorror))

(event Collision|EventActorBeginOverlap
  (params (OtherActor :type Actor%20Object%20Reference)))

(event EventTick
  (params (DeltaSeconds :type Float%20%28single-precision%29)))

(event EventApproach
  (params (Origin :type Actor%20Object%20Reference))
  (if (Variables|Default|GetCanInteract)
    (if (not (Variables|Default|GetInteracted))
      (Rendering|Material|SetOverlayMaterial (Variables|Default|GetStaticMesh) "/Game/Materials/InteractableHighlighter/MI_Highlight_Interactable.MI_Highlight_Interactable" :!class /Script/Engine.MeshComponent))))

(event EventLeave
  (Rendering|Material|SetOverlayMaterial (Variables|Default|GetStaticMesh) 0 :!class /Script/Engine.MeshComponent))

(event EventInteract
  (if (not (Variables|Default|GetbFixed))
    (bind _returnvalue (Actor|GetActorOfClass "/Game/Blueprints/BP_MasterManager.BP_MasterManager_C"))
    (Default|FixedPrinters _returnvalue)
    (Variables|Default|SetInteracted true)
    (Class|FMODAudioComponent|Stop (Variables|Default|GetFMODAudio))
    (Transformation|SetRelativeRotation (Variables|Default|GetDefaultSceneRoot) "0, 0, 0" false false)
    (bind _alpha (Timeline|Wiggle Stop)
      (:Update
        (Transformation|SetRelativeRotation (Variables|Default|GetDefaultSceneRoot) (Math|Rotator|Lerp(Rotator) "0.000000,0.000000,2.000000" "0.000000,0.000000,-2.000000" _alpha) false false)))))

(fn ConstructionScript)