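; BP_SoundTrigger is an interactable trigger box meant to play an FMOD event when BP_MainCharacter enters it.
; Box overlap calls PlayEventAtLocation at SoundPoint with AutoPlay off, so the returned instance is never started here, and prints a debug string.
; A HasPlayed flag limits this to one firing, and nothing happens when PlayOnce is false.
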(event OnComponentBeginOverlap(Box)
  (params (OverlappedComponent :type Primitive%20Component%20Object%20Reference) (OtherActor :type Actor%20Object%20Reference) (OtherComp :type Primitive%20Component%20Object%20Reference) (OtherBodyIndex :type Integer) (bFromSweep :type Boolean) (SweepResult :type Hit%20Result%20Structure%20%28by%20ref%29))
  (Utilities|Casting|CastToBP_MainCharacter OtherActor)
  (if (Variables|Default|GetbPlayOnce)
    (if (not (Variables|Default|GetbHasPlayed))
      (Development|PrintString "Played sound")
      (Class|FMODBlueprintStatics|PlayEventatLocation (Variables|Default|GetFMOD%20Event) (Math|Conversions|ToTransform(Vector) (Transformation|GetWorldLocation (Variables|Default|GetSoundPoint))) false)
      (Variables|Default|SetbHasPlayed true))))

(event EventBeginPlay)

(event Collision|EventActorBeginOverlap
  (params (OtherActor :type Actor%20Object%20Reference)))

(event EventTick
  (params (DeltaSeconds :type Float%20%28single-precision%29)))

(fn ConstructionScript)