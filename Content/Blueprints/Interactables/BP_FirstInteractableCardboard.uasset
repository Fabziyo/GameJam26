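; BP_FirstInteractableCardboard is a one-time interactable that triggers the first quest.
; Approach applies a highlight overlay material to the static mesh until the object has been used, and Leave clears it.
; The first Interact prints a placeholder animation message, sets the Interacted flag and calls FirstQuest on the BP_MasterManager found by class lookup.
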(event EventBeginPlay)

(event Collision|EventActorBeginOverlap
  (params (OtherActor :type Actor%20Object%20Reference)))

(event EventTick
  (params (DeltaSeconds :type Float%20%28single-precision%29)))

(event EventApproach
  (params (Origin :type Actor%20Object%20Reference))
  (if (not (Variables|Default|GetInteracted))
    (Rendering|Material|SetOverlayMaterial (Variables|Default|GetStaticMesh) "/Game/Materials/InteractableHighlighter/MI_Highlight_Interactable.MI_Highlight_Interactable" :!class /Script/Engine.MeshComponent)))

(event EventLeave
  (Rendering|Material|SetOverlayMaterial (Variables|Default|GetStaticMesh) 0 :!class /Script/Engine.MeshComponent))

(event EventInteract
  (if (not (Variables|Default|GetInteracted))
    (Development|PrintString "play anim")
    (Variables|Default|SetInteracted true)
    (bind _returnvalue (Actor|GetActorOfClass "/Game/Blueprints/BP_MasterManager.BP_MasterManager_C"))
    (Default|FirstQuest _returnvalue)))

(fn ConstructionScript)