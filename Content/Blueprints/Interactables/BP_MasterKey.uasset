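; BP_MasterKey is an interactable key pickup that the player collects, feeding a boss office check.
; Approach and Leave toggle a highlight overlay material on the key mesh.
; Interact adds the KeyID to the main character's collected keys, shows it as a timed message and plays FMOD audio.
; After a short delay it destroys itself, then sets Collected and calls BossOfficeCheck on the BP_MasterManager.
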(event EventBeginPlay)

(event Collision|EventActorBeginOverlap
  (params (OtherActor :type Actor%20Object%20Reference)))

(event EventTick
  (params (DeltaSeconds :type Float%20%28single-precision%29)))

(event EventApproach
  (params (Origin :type Actor%20Object%20Reference))
  (Rendering|Material|SetOverlayMaterial (Variables|Default|GetSM_Key) "/Game/Materials/InteractableHighlighter/MI_Highlight_Interactable.MI_Highlight_Interactable" :!class /Script/Engine.MeshComponent))

(event EventLeave
  (Rendering|Material|SetOverlayMaterial (Variables|Default|GetSM_Key) 0 :!class /Script/Engine.MeshComponent))

(event EventInteract
  (bind _asbp_main_character (Utilities|Casting|CastToBP_MainCharacter (Game|GetPlayerCharacter 0)))
  (Utilities|Array|AddUnique (Variables|/Game/Blueprint_Fabi/BP_MainCharacter.BP_MainCharacter_C|GetCollectedKeys _asbp_main_character) (Variables|Default|GetKeyID))
  (bind _asbp_main_character_2 (Utilities|Casting|CastToBP_MainCharacter (Game|GetPlayerCharacter 0)))
  (Default|ShowPlayerMessage _asbp_main_character_2 (Utilities|Text|ToText(Name) (Variables|Default|GetKeyID)) 2.5)
  (Class|FMODAudioComponent|Play (Variables|Default|GetFMODAudio))
  (Utilities|FlowControl|Delay 0.3)
  (Actor|DestroyActor)
  (Variables|Default|SetCollected true)
  (bind _returnvalue (Actor|GetActorOfClass "/Game/Blueprints/BP_MasterManager.BP_MasterManager_C"))
  (Default|BossOfficeCheck _returnvalue))

(fn ConstructionScript)