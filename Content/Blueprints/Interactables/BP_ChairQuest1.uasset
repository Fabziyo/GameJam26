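; BP_ChairQuest1 is an interactable chair for a quest, highlighted with an overlay material on approach while CanInteract is set.
; Interacting plays a timeline that lerps the actor from its current transform to TargetTransform, then marks it Placed.
; After short delays it triggers singing on BP_SoundWorkspace, then calls WorkSpaceQuest on BP_MasterManager, finding both by class lookup.
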(event EventBeginPlay)

(event Collision|EventActorBeginOverlap
  (params (OtherActor :type Actor%20Object%20Reference)))

(event EventTick
  (params (DeltaSeconds :type Float%20%28single-precision%29)))

(event EventApproach
  (params (Origin :type Actor%20Object%20Reference))
  (if (Variables|Default|GetbCanInteract)
    (Rendering|Material|SetOverlayMaterial (Variables|Default|GetSM_Interactable) "/Game/Materials/InteractableHighlighter/MI_Highlight_Interactable.MI_Highlight_Interactable" :!class /Script/Engine.MeshComponent)))

(event EventLeave
  (Rendering|Material|SetOverlayMaterial (Variables|Default|GetSM_Interactable) 0 :!class /Script/Engine.MeshComponent))

(event EventInteract
  (if (Variables|Default|GetbCanInteract)
    (Variables|Default|SetStartTransform (Transformation|GetActorTransform))
    (if (not (Variables|Default|GetbPlaced))
      (bind _alpha (Timeline|StuhlTransform Play)
        (:Update
          (Transformation|SetActorTransform (Math|Transform|Lerp(Transform) (Variables|Default|GetStartTransform) (Variables|Default|GetTargetTransform) _alpha)))
        (:Finished
          (Variables|Default|SetbPlaced true)
          (Utilities|FlowControl|Delay 0.75)
          (bind _returnvalue (Actor|GetActorOfClass "/Game/Blueprint_Fabi/BP_SoundWorkspace.BP_SoundWorkspace_C"))
          (Default|SoundPlaySinging _returnvalue)
          (Utilities|FlowControl|Delay 2.0)
          (bind _returnvalue_2 (Actor|GetActorOfClass "/Game/Blueprints/BP_MasterManager.BP_MasterManager_C"))
          (Default|WorkSpaceQuest _returnvalue_2))))))

(fn ConstructionScript)