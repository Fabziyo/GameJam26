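; BP_Kitchen is an interactable kitchen object that reveals the hidden BP_MasterKey after a set number of interactions.
; Approach and Leave toggle a highlight overlay on its mesh, and Interact counts uses while CanInteract is true.
; The matching interaction plays a timeline that rotates the root, then unhides the key, with a debug print standing in for its sound.
; Other interactions rotate it via a second timeline that reverses after a delay triggered from its Update pin.
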(event EventBeginPlay)

(event Collision|EventActorBeginOverlap
  (params (OtherActor :type Actor%20Object%20Reference)))

(event EventApproach
  (params (Origin :type Actor%20Object%20Reference))
  (if (Variables|Default|GetbCanInteract)
    (Rendering|Material|SetOverlayMaterial (Variables|Default|GetStaticMesh) "/Game/Materials/InteractableHighlighter/MI_Highlight_Interactable.MI_Highlight_Interactable" :!class /Script/Engine.MeshComponent)))

(event EventLeave
  (Rendering|Material|SetOverlayMaterial (Variables|Default|GetStaticMesh) 0 :!class /Script/Engine.MeshComponent))

(event EventTick
  (params (DeltaSeconds :type Float%20%28single-precision%29)))

(event EventInteract
  (if (Variables|Default|GetbCanInteract)
    (bind _output_get (Variables|Default|SetTimesInteracted (+ (Variables|Default|GetTimesInteracted) 1)))
    (if (== (Variables|Default|GetNeededInteraction) _output_get)
      (bind _alpha (Timeline|Timeline Play)
        (:Update
          (Transformation|SetRelativeRotation (Variables|Default|GetDefaultSceneRoot) (Math|Rotator|Lerp(Rotator) "0.000000,0.000000,0.000000" "-20.000000,0.000000,0.000000" _alpha) false false))
        (:Finished
          (Development|PrintString "Schlüsselsound auf Tisch")
          (bind _returnvalue (Actor|GetActorOfClass "/Game/Blueprints/Interactables/BP_MasterKey.BP_MasterKey_C"))
          (Rendering|SetActorHiddenInGame _returnvalue false)))
      (else
        (bind _alpha_2 (Timeline|Rotation Play)
          (:Update
            (Transformation|SetRelativeRotation (Variables|Default|GetDefaultSceneRoot) (Math|Rotator|Lerp(Rotator) "0.000000,0.000000,0.000000" "-20.000000,0.000000,0.000000" _alpha_2) false false)
            (Utilities|FlowControl|Delay 2.5)
            (Timeline|Rotation Reverse)))))))

(fn ConstructionScript)