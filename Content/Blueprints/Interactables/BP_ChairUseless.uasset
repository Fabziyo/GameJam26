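; BP_ChairUseless is an interactable chair that moves once to a target transform when used.
; Approach applies a highlight overlay material to its mesh while it is unplaced, and Leave clears it.
; Interact captures the current transform, then the StuhlTransform timeline lerps the actor to TargetTransform and sets Placed on finish, which blocks further highlighting and movement.
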(event EventBeginPlay)

(event Collision|EventActorBeginOverlap
  (params (OtherActor :type Actor%20Object%20Reference)))

(event EventTick
  (params (DeltaSeconds :type Float%20%28single-precision%29)))

(event EventApproach
  (params (Origin :type Actor%20Object%20Reference))
  (if (not (Variables|Default|GetbPlaced))
    (Rendering|Material|SetOverlayMaterial (Variables|Default|GetSM_Interactable) "/Game/Materials/InteractableHighlighter/MI_Highlight_Interactable.MI_Highlight_Interactable" :!class /Script/Engine.MeshComponent)))

(event EventLeave
  (Rendering|Material|SetOverlayMaterial (Variables|Default|GetSM_Interactable) 0 :!class /Script/Engine.MeshComponent))

(event EventInteract
  (Variables|Default|SetStartTransform (Transformation|GetActorTransform))
  (if (not (Variables|Default|GetbPlaced))
    (bind _alpha (Timeline|StuhlTransform PlayFromStart)
      (:Update
        (Transformation|SetActorTransform (Math|Transform|Lerp(Transform) (Variables|Default|GetStartTransform) (Variables|Default|GetTargetTransform) _alpha)))
      (:Finished
        (Variables|Default|SetbPlaced true)))))

(fn ConstructionScript)