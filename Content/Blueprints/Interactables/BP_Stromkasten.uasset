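; Interactable power box (Stromkasten) that turns on the lights when used.
; Interact, gated by CanInteract, finds all BP_LightManager actors, calls TurnOnAllLights, sets Interacted and prints a placeholder for the power-on sound.
; Approach applies a highlight overlay material while interactable and unused, and Leave clears it.
; Interacted only suppresses the highlight, not repeat use, and a PlayEvent2D node is left unconnected.
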(event EventBeginPlay)

(event Collision|EventActorBeginOverlap
  (params (OtherActor :type Actor%20Object%20Reference)))

(event EventTick
  (params (DeltaSeconds :type Float%20%28single-precision%29)))

(event EventApproach
  (params (Origin :type Actor%20Object%20Reference))
  (if (Variables|Default|GetbCanInteract)
    (if (not (Variables|Default|GetInteracted))
      (Rendering|Material|SetOverlayMaterial (Variables|Default|GetStaticMesh) "/Game/Materials/InteractableHighlighter/MI_Highlight_Interactable.MI_Highlight_Interactable" :!class /Script/Engine.MeshComponent))))

(event EventLeave
  (Rendering|Material|SetOverlayMaterial (Variables|Default|GetStaticMesh) 0 :!class /Script/Engine.MeshComponent))

(event EventInteract
  (if (Variables|Default|GetbCanInteract)
    (bind _outactors (Actor|GetAllActorsOfClass "/Game/Blueprints/Lamp/BP_LightManager.BP_LightManager_C"))
    (Default|TurnonAllLights _outactors)
    (Variables|Default|SetInteracted true)
    (Development|PrintString "Play Sound: Strom an")))

(fn ConstructionScript)