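; BP_EndGame is a trigger box that runs the game's ending sequence when overlapped.
; After a short delay and a DoOnce, it casts to BP_MainCharacter, so any first overlapping actor consumes the trigger.
; It disables the player's movement and flashlight, then plays a fade-to-black widget and a placeholder jumpscare print.
; It then shows the end screen with UI-only input and cursor, and later opens the main menu level.
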(event OnComponentBeginOverlap(Box)
  (params (OverlappedComponent :type Primitive%20Component%20Object%20Reference) (OtherActor :type Actor%20Object%20Reference) (OtherComp :type Primitive%20Component%20Object%20Reference) (OtherBodyIndex :type Integer) (bFromSweep :type Boolean) (SweepResult :type Hit%20Result%20Structure%20%28by%20ref%29))
  (bind _returnvalue (Game|GetPlayerController 0))
  (Utilities|FlowControl|Delay 0.3)
  (Utilities|FlowControl|DoOnce false
    (:Completed
      (bind _asbp_main_character (Utilities|Casting|CastToBP_MainCharacter OtherActor))
      (Pawn|Components|CharacterMovement|DisableMovement (Variables|/Script/Engine.Character|GetCharacterMovement _asbp_main_character))
      (Variables|/Game/Blueprint_Fabi/BP_MainCharacter.BP_MainCharacter_C|SetbCanUseFlashlight _asbp_main_character false)
      (Rendering|SetVisibility (Variables|/Game/Blueprint_Fabi/BP_MainCharacter.BP_MainCharacter_C|GetFlashlight _asbp_main_character) false false)
      (Utilities|FlowControl|Delay 0.5)
      (bind _returnvalue_2 (UserInterface|CreateWidget "/Game/UI/WBP_FadeToBlack.WBP_FadeToBlack_C"))
      (UserInterface|Viewport|AddtoViewport _returnvalue_2 0)
      (UserInterface|Animation|PlayAnimation _returnvalue_2 (Variables|/Game/UI/WBP_FadeToBlack.WBP_FadeToBlack_C|GetFadeToBlack _returnvalue_2) 0.0 1 "Forward" 1.0 false)
      (Utilities|FlowControl|Delay 2.5)
      (Development|PrintString "Play Jumpscare")
      (Utilities|FlowControl|Delay 3.0)
      (bind _returnvalue_3 (UserInterface|CreateWidget "/Game/UI/WBP_EndScreen.WBP_EndScreen_C"))
      (UserInterface|Viewport|AddtoViewport _returnvalue_3 0)
      (Input|SetInputModeUIOnly _returnvalue _returnvalue_3 "DoNotLock" false)
      (Variables|/Script/Engine.PlayerController|SetbShowMouseCursor _returnvalue true)
      (Utilities|FlowControl|Delay 2e+01)
      (Game|OpenLevel(byObjectReference) "/Game/Levels/L_MainMenu.L_MainMenu"))))

(event EventBeginPlay)

(event Collision|EventActorBeginOverlap
  (params (OtherActor :type Actor%20Object%20Reference)))

(event EventTick
  (params (DeltaSeconds :type Float%20%28single-precision%29)))

(fn ConstructionScript)