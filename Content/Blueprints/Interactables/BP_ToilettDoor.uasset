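; Interactable toilet door that highlights on approach while interaction is allowed and can trigger an optional jumpscare.
; Interact plays the DoorRotate timeline to swing the mesh open, and once Interacted is set, later interactions reverse it.
; With Jumpscare enabled, delayed calls chained off the timeline update play a one-shot FMOD sound, then call WiggleHorror on BP_MasterManager.
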(event Custom|Sound%20Jumpscare
  (if (Variables|Default|GetJumpscare)
    (Utilities|FlowControl|DoOnce false
      (:Completed
        (Class|FMODAudioComponent|Play (Variables|Default|GetFMODAudio))))))

(event EventBeginPlay)

(event Collision|EventActorBeginOverlap
  (params (OtherActor :type Actor%20Object%20Reference)))

(event EventTick
  (params (DeltaSeconds :type Float%20%28single-precision%29)))

(event EventApproach
  (params (Origin :type Actor%20Object%20Reference))
  (if (Variables|Default|GetbcanInteract)
    (Rendering|Material|SetOverlayMaterial (Variables|Default|GetStaticMesh1) "/Game/Materials/InteractableHighlighter/MI_Highlight_Interactable.MI_Highlight_Interactable" :!class /Script/Engine.MeshComponent)))

(event EventLeave
  (Rendering|Material|SetOverlayMaterial (Variables|Default|GetStaticMesh1) 0 :!class /Script/Engine.MeshComponent))

(event EventInteract
  (if (Variables|Default|GetbcanInteract)
    (if (not (Variables|Default|GetInteracted))
      (bind _alpha (Timeline|DoorRotate Play)
        (:Update
          (Transformation|SetRelativeRotation (Variables|Default|GetStaticMesh) (Math|Rotator|Lerp(Rotator) "0, 0, 0" "0.000000,-90.000000,0.000000" _alpha) false false)
          (Variables|Default|SetInteracted true)
          (Utilities|FlowControl|Delay 0.75)
          (if (Variables|Default|GetJumpscare)
            (CallFunction|SoundJumpscare)
            (Utilities|FlowControl|Delay 0.5)
            (bind _returnvalue (Actor|GetActorOfClass "/Game/Blueprints/BP_MasterManager.BP_MasterManager_C"))
            (Default|WiggleHorror _returnvalue))))
      (else
        (Timeline|DoorRotate Reverse)))))

(fn ConstructionScript)