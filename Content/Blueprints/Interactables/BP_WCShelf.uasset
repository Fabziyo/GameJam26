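; BP_WCShelf is an interactable shelf whose thirteen static mesh pieces are knocked loose when the player walks into its trigger box.
; On box overlap, it turns on physics for every piece and applies one strong force along world X to throw them.
; A DoOnce runs before the player character check, so the first overlap by any actor uses up the one-shot, even if nothing falls.
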(event OnComponentBeginOverlap(Box)
  (params (OverlappedComponent :type Primitive%20Component%20Object%20Reference) (OtherActor :type Actor%20Object%20Reference) (OtherComp :type Primitive%20Component%20Object%20Reference) (OtherBodyIndex :type Integer) (bFromSweep :type Boolean) (SweepResult :type Hit%20Result%20Structure%20%28by%20ref%29))
  (Utilities|FlowControl|DoOnce false
    (:Completed
      (if (== OtherActor (Game|GetPlayerCharacter 0))
        (Physics|SetSimulatePhysics (Variables|Default|GetStaticMesh1) true)
        (Physics|AddForce (Variables|Default|GetStaticMesh3) "90000.000000,0.000000,0.000000" "None" false)))))

(event EventBeginPlay)

(event Collision|EventActorBeginOverlap
  (params (OtherActor :type Actor%20Object%20Reference)))

(event EventTick
  (params (DeltaSeconds :type Float%20%28single-precision%29)))

(fn ConstructionScript)