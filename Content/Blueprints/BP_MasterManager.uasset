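; BP_MasterManager drives the linear quest chain of an office horror game, from the instruction board through printers, kitchen and power outage to leaving the building.
; Each quest event sets the step and objective text, then finds actors by class to enable interaction or trigger ghosts, sounds and lights.
; Quests are started by external calls, except the kitchen quest, which follows once enough printers are fixed.
; It also grants key IDs to the player.
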(event Custom|StartGameEvent
  ;[0.15 0.15 0.15 0.5] Game start
  (Variables|Default|SetCurrentStep 0)
  (Variables|Default|SetCurrentObjective "Check the instructions on the board."))

(event Custom|TriggerStromausfall
  ;[0.15 0.15 0.15 0.5] Stromausfall-Quest
  (bind _returnvalue (Actor|GetActorOfClass "/Game/Blueprints/Lamp/BP_LightManager.BP_LightManager_C"))
  (Default|TurnOffAllLights _returnvalue)
  (Variables|Default|SetbPowerIsOut true)
  (Variables|Default|SetbStromkastenAvailable true)
  (Variables|Default|SetCurrentStep 9)
  (Variables|Default|SetCurrentObjective "Restore the power in the basement.")
  (CallFunction|SoundPlayImpactHeavy))

(event Custom|FirstQuest
  ;[0.15 0.15 0.15 0.5] Versammlungsraum-Quest
  (Variables|Default|SetCurrentStep 1)
  (Variables|Default|SetCurrentObjective "Check the office")
  (bind _returnvalue (Actor|GetActorOfClass "/Game/Blueprints/Interactables/BP_ChairQuest1.BP_ChairQuest1_C"))
  (Variables|/Game/Blueprints/Interactables/BP_ChairQuest1.BP_ChairQuest1_C|SetbCanInteract _returnvalue true)
  (bind _returnvalue_2 (Actor|GetActorOfClass "/Game/Blueprints/Interactables/BP_ChairUseless.BP_ChairUseless_C"))
  (Variables|/Game/Blueprints/Interactables/BP_ChairUseless.BP_ChairUseless_C|SetbCanInteract _returnvalue_2 true)
  (CallFunction|GhostStandAlone))

(event Custom|GivePlayerKey
  (params (KeyID :type Name))
  (bind _asbp_main_character (Utilities|Casting|CastToBP_MainCharacter (Game|GetPlayerCharacter 0)))
  (Utilities|Array|AddUnique (Variables|/Game/Blueprint_Fabi/BP_MainCharacter.BP_MainCharacter_C|GetCollectedKeys _asbp_main_character) KeyID))

(event Custom|Ghost%20StandAlone
  (bind _returnvalue (Actor|GetActorOfClass "/Game/Blueprint_Fabi/BP_Geist_Jumpscare_Standalone.BP_Geist_Jumpscare_Standalone_C"))
  (Default|TriggeronStandAlone _returnvalue))

(event Custom|Sound%20Play%20laugh
  (bind _returnvalue (Actor|GetActorOfClass "/Game/Blueprint_Fabi/BP_Sound.BP_Sound_C"))
  (Default|SoundPlayLaughing _returnvalue))

(event Custom|Sound%20Play%20Sing
  (bind _returnvalue (Actor|GetActorOfClass "/Game/Blueprint_Fabi/BP_Sound2.BP_Sound2_C"))
  (Default|SoundPlaySinging _returnvalue))

(event Custom|Sound%20Play%20Scream
  (bind _returnvalue (Actor|GetActorOfClass "/Game/Blueprint_Fabi/BP_Sound3.BP_Sound3_C"))
  (Default|SoundPlayScreaming _returnvalue))

(event Custom|Sound%20Play%20Impact%20Heavy
  (bind _returnvalue (Actor|GetActorOfClass "/Game/Blueprint_Fabi/BP_Sound4.BP_Sound4_C"))
  (Default|SoundPlayImpact _returnvalue))

(event Custom|RestorePower
  ;[0.15 0.15 0.15 0.5] Stromausfall-Quest
  (CallFunction|SoundPlayScream)
  (Variables|Default|SetbPowerIsOut false)
  (Variables|Default|SetbStromkastenAvailable false)
  (Variables|Default|SetCurrentStep 10)
  (Variables|Default|SetCurrentObjective "Leave the Building!")
  (bind _returnvalue (Actor|GetActorOfClass "/Game/Blueprints/Lamp/BP_LightManager.BP_LightManager_C"))
  (Default|TurnonAllLights _returnvalue))

(event Custom|GhostWorkspace
  ;[0.15 0.15 0.15 0.5] Workspace-Quest
  (bind _returnvalue (Actor|GetActorOfClass "/Game/Blueprint_Fabi/BP_Geist.BP_Geist_C"))
  (Default|SetTriggeronWorkspace _returnvalue)
  (Utilities|FlowControl|Delay 3.0)
  (Variables|Default|SetCurrentStep 3)
  (Utilities|FlowControl|Delay 1.5))

(event Custom|WiggleHorror
  ;[0.15 0.15 0.15 0.5] Wiggling Printers Quest
  (bind _outactors (Actor|GetAllActorsOfClass "/Game/Blueprints/Interactables/BP_Printer.BP_Printer_C"))
  (for _array_element _outactors
    (Default|WiggleHorror _array_element))
  (Variables|Default|SetCurrentStep 5)
  (Variables|Default|SetCurrentObjective "Deactivate the printers."))

(event Custom|FixedPrinters
  ;[0.15 0.15 0.15 0.5] Wiggling Printers Quest
  (bind _output_get (Variables|Default|SetPrintersFixed (+ (Variables|Default|GetPrintersFixed) 1)))
  (if (>= _output_get (Variables|Default|GetRequiredPrinters))
    (Variables|Default|SetCurrentStep 6)
    (Utilities|FlowControl|Delay 1.0)
    (CallFunction|KitchenQuest)
    (CallFunction|SoundPlaySing)))

(event Custom|Toilette
  ;[0.15 0.15 0.15 0.5] Bathroom Quest
  (Utilities|FlowControl|Delay 1.5)
  (Variables|Default|SetCurrentStep 4)
  (Variables|Default|SetCurrentObjective "Check where that thing went.")
  (bind _outactors (Actor|GetAllActorsOfClass "/Game/Blueprints/Interactables/BP_ToilettDoor.BP_ToilettDoor_C"))
  (for _array_element _outactors
    (Variables|/Game/Blueprints/Interactables/BP_ToilettDoor.BP_ToilettDoor_C|SetbcanInteract _array_element true)))

(event Custom|WorkSpaceQuest
  ;[0.15 0.15 0.15 0.5] Workspace-Quest
  (Variables|Default|SetCurrentStep 2)
  (Variables|Default|SetCurrentObjective "Check the workspace.")
  (CallFunction|GhostWorkspace))

(event Custom|KitchenQuest
  ;[0.15 0.15 0.15 0.5] Kitchen Quest
  (Variables|Default|SetCurrentStep 7)
  (Variables|Default|SetCurrentObjective "Check the noises in the kitchen")
  (bind _returnvalue (Actor|GetActorOfClass "/Game/Blueprints/Interactables/BP_Kitchen.BP_Kitchen_C"))
  (Variables|/Game/Blueprints/Interactables/BP_Kitchen.BP_Kitchen_C|SetbCanInteract _returnvalue true))

(event Custom|BossOfficeCheck
  ;[0.15 0.15 0.15 0.5] Boss office Quest
  (Variables|Default|SetCurrentStep 8)
  (Variables|Default|SetCurrentObjective "Check the boss office")
  (CallFunction|SoundPlayLaugh))

(event EventBeginPlay
  (CallFunction|StartGameEvent))

(event Collision|EventActorBeginOverlap
  (params (OtherActor :type Actor%20Object%20Reference)))

(event EventTick
  (params (DeltaSeconds :type Float%20%28single-precision%29)))

(fn ConstructionScript)