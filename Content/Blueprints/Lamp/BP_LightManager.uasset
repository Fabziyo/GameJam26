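; BP_LightManager is a manager Blueprint that switches every RectLight actor in the level on or off.
; Two custom events, TurnOnAllLights and TurnOffAllLights, gather all RectLight actors with GetAllActorsOfClass and set each light component's visibility.
; Begin play, tick, overlap and construction script are empty, and a tag-based component lookup is left unconnected.
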(event Custom|TurnOffAllLights
  (bind _outactors (Actor|GetAllActorsOfClass "/Script/Engine.RectLight"))
  (for _array_element _outactors
    (Rendering|SetVisibility (Variables|/Script/Engine.RectLight|GetRectLightComponent _array_element) false false)))

(event Custom|TurnOnAllLights
  (bind _outactors (Actor|GetAllActorsOfClass "/Script/Engine.RectLight"))
  (for _array_element _outactors
    (Rendering|SetVisibility (Variables|/Script/Engine.RectLight|GetRectLightComponent _array_element) true false)))

(event EventBeginPlay)

(event Collision|EventActorBeginOverlap
  (params (OtherActor :type Actor%20Object%20Reference)))

(event EventTick
  (params (DeltaSeconds :type Float%20%28single-precision%29)))

(fn ConstructionScript)