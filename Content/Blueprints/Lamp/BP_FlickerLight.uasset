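; Flickering rect light actor that randomizes its intensity from BeginPlay onward.
; Flicker re-calls itself after a random delay, picking an intensity between BaseIntensity and FlickerStrength.
; BeginPlay also starts a looping timer with a period randomized once, though its bound event is not named.
; A Blackout event prints a debug message, spikes the light, cuts it to dark, then restores base intensity, without pausing the flicker loop.
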(event Custom|Flicker
  (Rendering|Components|Light|SetIntensity (Variables|Default|GetRectLight) (Math|Random|RandomFloatinRange (Variables|Default|GetBaseIntensity) (Variables|Default|GetFlickerStrength)))
  (Utilities|FlowControl|Delay (Math|Random|RandomFloatinRange (Variables|Default|GetMinDelay) (Variables|Default|GetMaxDelay)))
  (CallFunction|Flicker))

(event Custom|Blackout
  (Development|PrintString "Blackout!")
  (Rendering|Components|Light|SetIntensity (Variables|Default|GetRectLight) 1e+02)
  (Utilities|FlowControl|Delay 0.1)
  (Rendering|Components|Light|SetIntensity (Variables|Default|GetRectLight) 0.0)
  (Utilities|FlowControl|Delay 1.5)
  (Rendering|Components|Light|SetIntensity (Variables|Default|GetRectLight) (Variables|Default|GetBaseIntensity)))

(event EventBeginPlay
  (CallFunction|Flicker)
  (Utilities|Time|SetTimerbyEvent (EventDispatchers|CreateEvent :!event Custom|Blackout) (Math|Random|RandomFloatinRange 2e+01 6e+01) true))

(event Collision|EventActorBeginOverlap
  (params (OtherActor :type Actor%20Object%20Reference)))

(event EventTick
  (params (DeltaSeconds :type Float%20%28single-precision%29)))

(fn ConstructionScript)