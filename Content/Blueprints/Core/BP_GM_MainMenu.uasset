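; Main menu game mode that brings up the front-end UI and music when the menu level starts.
; On BeginPlay it creates the core UI widget, adds it to the viewport and pushes the main menu root onto its menu stack.
; It switches the first player to UI-only input with a visible cursor, then starts playback on an FMOD audio component.
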(event Custom|SetUpUI
  (bind _returnvalue (Game|GetPlayerController 0))
  (bind _returnvalue_2 (UserInterface|CreateWidget "/Game/UI/WBP_CoreUI.WBP_CoreUI_C"))
  (bind _output_get (Variables|Default|SetCoreUI _returnvalue_2))
  (UserInterface|Viewport|AddtoViewport _output_get 0)
  (Class|CommonActivatableWidgetContainerBase|AddWidget (Variables|/Game/UI/WBP_CoreUI.WBP_CoreUI_C|GetMainMenuStack _output_get) "/Game/UI/MainMenu/WBP_MainMenuRoot.WBP_MainMenuRoot_C")
  (Input|SetInputModeUIOnly _returnvalue 0 "DoNotLock" false)
  (Variables|/Script/Engine.PlayerController|SetbShowMouseCursor _returnvalue true))

(event Custom|Play%20Track
  (Class|FMODAudioComponent|Play (Variables|Default|GetFMODAudio)))

(event EventBeginPlay
  (CallFunction|SetUpUI)
  (CallFunction|PlayTrack))

(event EventTick
  (params (DeltaSeconds :type Float%20%28single-precision%29)))

(fn ConstructionScript)