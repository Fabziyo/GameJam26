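; BP_GMGame is the game mode that handles music, UI setup, player respawning and pausing.
; On BeginPlay it caches a PlayerStart transform, creates the core UI with gameplay UI on its widget stack, and starts looped ambient music.
; PlayerSpawn restarts the player at that transform, which SetPlayerRespawnPoint can overwrite, with a camera fade.
; PauseMenu toggles pause, using a separate widget stack and switching input mode and cursor.
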(event Custom|SetupUI
  ;[0.15 0.15 0.15 0.5] SetupUI
  (bind _returnvalue (UserInterface|CreateWidget "/Game/UI/WBP_CoreUI.WBP_CoreUI_C"))
  (bind _output_get (Variables|Default|SetCore%20UI _returnvalue))
  (UserInterface|Viewport|AddtoViewport _output_get 0)
  (bind _returnvalue_2 (Class|CommonActivatableWidgetContainerBase|AddWidget (Variables|/Game/UI/WBP_CoreUI.WBP_CoreUI_C|GetGameplayStack _output_get) "/Game/UI/WBP_GameplayUI.WBP_GameplayUI_C"))
  (Variables|Default|SetGameplayUI _returnvalue_2))

(event Custom|SetupPlayerSpawn
  ;[0.15 0.15 0.15 0.5] SetupPlayerSpawn
  (bind _returnvalue (Actor|GetActorOfClass "/Script/Engine.PlayerStart"))
  (Variables|Default|SetPlayer%20Spawn%20Transform (Transformation|GetActorTransform _returnvalue)))

(event Custom|Event%20PlayerSpawn
  (bind _player_spawn_transform (Variables|Default|GetPlayer%20Spawn%20Transform))
  ;[0.15 0.15 0.15 0.5] PlayerSpawn
  (Class|GameModeBase|RestartPlayeratTransform (Game|GetPlayerController 0) (Math|Transform|MakeTransform (.location _player_spawn_transform) (.rotation _player_spawn_transform) "1.000000,1.000000,1.000000"))
  (CameraFades|StartCameraFade :self (Game|GetPlayerCameraManager 0) :FromAlpha 1.0 :Duration 2.0))

(event Custom|Play%20Music
  (Class|FMODBlueprintStatics|PlayEvent2D "/Game/FMOD/Events/Music/DarkAmbients_looped_.DarkAmbients_looped_"))

(event EventBeginPlay
  (CallFunction|SetupPlayerSpawn)
  (CallFunction|SetupUI)
  (CallFunction|PlayMusic))

(event EventTick
  (params (DeltaSeconds :type Float%20%28single-precision%29)))

(event EventPauseMenu
  (bind _returnvalue (Game|GetPlayerController 0))
  (bind _returnvalue_2 (Game|GetPlayerController 0))
  ;[0.15 0.15 0.15 0.5] PauseMenu
  (if (not (Game|IsGamePaused))
    (Class|CommonActivatableWidgetContainerBase|AddWidget (Variables|/Game/UI/WBP_CoreUI.WBP_CoreUI_C|GetPauseStack (Variables|Default|GetCore%20UI)) "/Game/UI/WBP_PauseMenuRoot.WBP_PauseMenuRoot_C")
    (Game|SetGamePaused true)
    (Input|SetInputModeUIOnly _returnvalue_2 0 "DoNotLock" false)
    (Variables|/Script/Engine.PlayerController|SetbShowMouseCursor _returnvalue_2 true)
    (else
      (Class|CommonActivatableWidgetContainerBase|ClearWidgets (Variables|/Game/UI/WBP_CoreUI.WBP_CoreUI_C|GetPauseStack (Variables|Default|GetCore%20UI)))
      (Game|SetGamePaused false)
      (Input|SetInputModeGameOnly _returnvalue false)
      (Variables|/Script/Engine.PlayerController|SetbShowMouseCursor _returnvalue false))))

(event EventSetPlayerRespawnPoint
  (params (NewTransform :type Transform))
  ;[0.15 0.15 0.15 0.5] PlayerSpawnRespawn
  (Variables|Default|SetPlayer%20Spawn%20Transform NewTransform))

(fn ConstructionScript)